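; Gun actor that auto-fires bullets from the moment it begins play until ReleaseTrigger stops it.
; BeginPlay fires once, then loops Attach on a timer whose interval is the reciprocal of BulletVelocity, so that variable acts as fire rate.
; Each Attach spawns a short-lived Bp_Wp_Bullet_002 at the Arrow transform, with pistol sound and muzzle effect at the actor's location.
; IsPlayer always returns false.
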(event `self.ReceiveBeginPlay`
  (`self.Attach`)
  (`KismetSystemLibrary.K2_SetTimer` null "Attach" (/ 1.0 (`self.Bullet Velocity`)) true))

(event `ReleaseTrigger`
  (`KismetSystemLibrary.K2_ClearTimer` null "Attach"))

(fn `Attach`
  (bind _returnvalue (`|SpawnActorFromClass` "/Game/Blueprints/Bullet/Bp_Wp_Bullet_002.Bp_Wp_Bullet_002_C" (`SceneComponent.K2_GetComponentToWorld` (`self.Arrow`)) "AlwaysSpawn" "MultiplyWithRoot" null null))
  (`self.SetLifeSpan` _returnvalue 2.0)
  (`GameplayStatics.SpawnSoundAtLocation` "/Game/Sound/Weapon/Pistiol/Pistol_shot.Pistol_shot" (`self.K2_GetActorLocation`) (`self.K2_GetActorRotation`) 1.0 1.0 0.0 null null)
  (`GameplayStatics.SpawnEmitterAtLocation` "/Game/Effects/Particles/P_Fx_BLT_Muzzle.P_Fx_BLT_Muzzle" (`self.K2_GetActorLocation`) (`self.K2_GetActorRotation`) (0.3 0.3 0.3)) ; 发射时特效
)

(fn `IsPlayer`
  (returns (Player :type Boolean))
  (return false))

(fn `UserConstructionScript`)