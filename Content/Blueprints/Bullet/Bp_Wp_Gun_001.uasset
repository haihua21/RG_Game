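; Hitscan automatic gun that starts firing on BeginPlay and repeats on a looping timer, with BulletVelocity as shots per second, until ReleaseTrigger clears it.
; Each shot runs in Attach, which plays sound and muzzle effects, sphere-traces forward and draws a Niagara tracer to the impact or trace end.
; Hits spawn an impact effect and send Damage through WeaponMessage to actors implementing BpI_Character.
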(event `self.ReceiveBeginPlay`
  (`self.Attach`)
  (`KismetSystemLibrary.K2_SetTimer` null "Attach" (/ 1.0 (`self.Bullet Velocity`)) true))

(event `ReleaseTrigger`
  (`KismetSystemLibrary.K2_ClearTimer` null "Attach"))

(fn `Attach`
  (bind _returnvalue (`self.K2_GetActorLocation`))
  (bind _returnvalue_2 (`self.K2_GetActorRotation`))
  (bind _returnvalue_3 (`self.K2_GetActorLocation`))
  (bind _returnvalue_4 (+ (* (`self.GetActorForwardVector`) 1000) _returnvalue_3))
  (`GameplayStatics.SpawnSoundAtLocation` "/Game/Sound/Weapon/Pistiol/Pistol_shot.Pistol_shot" (`self.K2_GetActorLocation`) (`self.K2_GetActorRotation`) 1.0 1.0 0.0 null null)
  (bind (_outhit _returnvalue_5) (`KismetSystemLibrary.SphereTraceSingleForObjects` :`Start` _returnvalue_3 :`End` _returnvalue_4 :`Radius` 0.1 :`ObjectTypes` (`self.Object Types`) :`DrawTime` 1.0))
  (`GameplayStatics.SpawnEmitterAtLocation` "/Game/Effects/Particles/P_Fx_BLT_Muzzle.P_Fx_BLT_Muzzle" (`self.K2_GetActorLocation`) _returnvalue_2 (0.3 0.3 0.3)) ; 发射时特效
  (bind _returnvalue_6 (`NiagaraFunctionLibrary.SpawnSystemAtLocation` "/Game/Effects/Niagara/NS_bulletTrace.NS_bulletTrace" _returnvalue _returnvalue_2)) ; 过程中
  (`NiagaraComponent.SetVariablePosition` _returnvalue_6 "start" _returnvalue)
  (if _returnvalue_5
    (bind (_bblockinghit _binitialoverlap _time _distance _location _impactpoint _normal _impactnormal _physmat _hitactor) (`GameplayStatics.BreakHitResult` _outhit))
    (`NiagaraComponent.SetVariablePosition` _returnvalue_6 "end" _impactpoint)
    (`GameplayStatics.SpawnEmitterAtLocation` "/Game/Effects/Particles/P_Fx_hudun_x_sj.P_Fx_hudun_x_sj" _impactpoint (struct) (0.3 0.3 0.3)) ; 击中后 增加特效
    (if (`KismetSystemLibrary.DoesImplementInterface` _hitactor "/Game/Blueprints/Data/BpI_Character.BpI_Character_C")
      (message `/Game/Blueprints/Data/BpI_Character.Weapon` _hitactor (`self.Damage`)))
    (else
      (`NiagaraComponent.SetVariablePosition` _returnvalue_6 "end" _returnvalue_4))))

(fn `IsPlayer`
  (returns (Player :type Boolean))
  (return false))

(fn `UserConstructionScript`)