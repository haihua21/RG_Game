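; Basic bullet actor that detects and affects NPC characters with a forward sphere trace.
; Every Tick, Attach replays the shot sound and muzzle effects, then runs a short debug-drawn trace.
; Trace hits spawn an emitter at the impact normal (not point), call CusNpcAffected on NPCs, then write Damage to the Dt_Game_State game instance.
; Sphere collisions with non-NPCs destroy the bullet; effect start/end parameter setters are disconnected.
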(event `self.ReceiveBeginPlay`
  (bind _asdt_game_state (cast `/Game/Blueprints/Data/Dt_Game_State` (`GameplayStatics.GetGameInstance`)))
  (set `self.As Dt Game State` _asdt_game_state))

(event `self.ReceiveTick`
  (params (DeltaSeconds :type "Float (single-precision)"))
  (`self.Attach`))

(event `self.Sphere.OnComponentHit`
  (params (HitComponent :type "PrimitiveComponent Object Reference") (OtherActor :type "Actor Object Reference") (OtherComp :type "PrimitiveComponent Object Reference") (NormalImpulse :type "Vector Structure") (Hit :type "HitResult Structure (by ref)"))
  (cast `/Game/Blueprints/Npc/Bp_Npc_TopDownCharacter_Child` OtherActor
    (:`CastFailed`
      (`self.K2_DestroyActor`))))

(fn `Attach`
  (bind _returnvalue (`self.K2_GetActorRotation`))
  (bind _returnvalue_2 (`self.K2_GetActorLocation`))
  (`GameplayStatics.SpawnSoundAtLocation` "/Game/Sound/Weapon/Pistiol/shot_1.shot_1" (`self.K2_GetActorLocation`) (`self.K2_GetActorRotation`) 1.0 1.0 0.0 null null)
  (bind (_outhit _returnvalue_3) (`KismetSystemLibrary.SphereTraceSingleForObjects` :`Start` _returnvalue_2 :`End` (+ (* (`self.GetActorForwardVector`) 500) _returnvalue_2) :`Radius` 5.0 :`ObjectTypes` (`self.Object Types`) :`DrawDebugType` "ForDuration" :`DrawTime` 2.0))
  (`GameplayStatics.SpawnEmitterAtLocation` null (`self.K2_GetActorLocation`) _returnvalue) ; 发射时特效
  (bind _returnvalue_4 (`NiagaraFunctionLibrary.SpawnSystemAtLocation` null (`self.K2_GetActorLocation`) _returnvalue))
  (if _returnvalue_3
    (bind (_bblockinghit _binitialoverlap _time _distance _location _impactpoint _normal _impactnormal _physmat _hitactor) (`GameplayStatics.BreakHitResult` _outhit))
    (`GameplayStatics.SpawnEmitterAtLocation` null _impactnormal) ; 击中后 增加特效
    (bind _asbp_npc_top_down_character_child (cast `/Game/Blueprints/Npc/Bp_Npc_TopDownCharacter_Child` _hitactor))
    (`/Game/Blueprints/Npc/Bp_Npc_TopDownCharacter_Child.Cus_Npc_Affected` _asbp_npc_top_down_character_child)
    (set `/Game/Blueprints/Data/Dt_Game_State.Damage` (`self.Damage`) (`self.As Dt Game State`))))

(fn `UserConstructionScript`)