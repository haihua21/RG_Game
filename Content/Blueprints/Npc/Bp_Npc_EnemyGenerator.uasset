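; Enemy spawner actor that creates AI characters at random points inside its Box volume.
; Each call to its EnemyGenerator event spawns one Bp_Npc_TopDownCharacter_Master while the live count is below MaxEnemyCount and LoopNumber is below NumberOfTimes.
; The live count only includes Bp_Npc_TopDownCharacter_Child actors, although the spawned class is the Master.
; LoopNumber tracks total spawns, and the trailing one-second Delay leads to no further logic.
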(event `EnemyGenerator`
  (bind _box (`self.Box`))
  (bind _outactors (`GameplayStatics.GetAllActorsOfClass` "/Game/Blueprints/Npc/Bp_Npc_TopDownCharacter_Child.Bp_Npc_TopDownCharacter_Child_C"))
  (if (< (`KismetArrayLibrary.Array_Length` _outactors) (`self.MaxEnemyCount`))
    (if (< (`self.LoopNumber`) (`self.NumberOfTimes`))
      (`|ExecutionSequence`
        (:`then_0`
          (`AIBlueprintHelperLibrary.SpawnAIFromClass` "/Game/Blueprints/Npc/Bp_Npc_TopDownCharacter_Master.Bp_Npc_TopDownCharacter_Master_C" null (`KismetMathLibrary.RandomPointInBoundingBox` (`SceneComponent.K2_GetComponentLocation` _box) (`BoxComponent.GetScaledBoxExtent` _box)) (struct) false null)
          (bind _result (`/Engine/EditorBlueprintResources/StandardMacros.IncrementInt` (`self.LoopNumber`))
            (:`  `
              (set `self.LoopNumber` _result)
              (`KismetSystemLibrary.Delay` 1.0))))))))

(fn `UserConstructionScript`)