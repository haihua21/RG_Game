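; Master NPC AI controller that makes its pawn follow a player detected through AI Perception.
; A successfully sensed actor that passes the IsPlayer interface check becomes Target and starts a self-repeating follow event on a short delay.
; Each pass issues AI MoveTo when the pawn is beyond a small distance, with a DoOnce blocking new moves until success or failure.
; Target is never cleared when sensing is lost.
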(event `Cus_AI_FollowTarget`
  (bind _target (`self.Target`))
  (`/Engine/EditorBlueprintResources/StandardMacros.IsValid` _target
    (:`Is Valid`
      (`|ExecutionSequence`
        (:`then_0`
          (`KismetSystemLibrary.Delay` 2.0)
          (`self.Cus_AI_FollowTarget`))
        (:`then_1`
          (if (> (`self.GetDistanceTo` _target (`self.K2_GetPawn`)) 50.0)
            (`/Engine/EditorBlueprintResources/StandardMacros.DoOnce` false :!label _label
              (:`Completed`
                (`|AIMoveTo` null (0.0 0.0 0.0) _target 20.0
                  (:`OnSuccess`
                    (goto _label :!via `Reset`))
                  (:`OnFail`
                    (goto _label :!via `Reset`)))))))))))

(event `self.AIPerception.OnTargetPerceptionUpdated`
  (params (Actor :type "Actor Object Reference") (Stimulus :type "AIStimulus Structure"))
  (bind _player (message `/Game/Blueprints/Data/BpI_Character.IsPlayer` Actor))
  (if _player
    (if (`.bSuccessfullySensed` (break `AIStimulus` Stimulus))
      (set `self.Target` Actor)
      (`self.Cus_AI_FollowTarget`))))

(fn `UserConstructionScript`)