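; Dropped XP pickup that spins at a slightly randomized rate and grants its XP to the top-down player character on overlap, then destroys itself.
; Two events move it after a delay, toward either a given location or the Target actor's position sampled once when the delay ends.
; Each uses a timeline to lerp from the current location every update rather than from a fixed start.
; A pickup emitter spawn is present but unconnected.
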(event `self.ReceiveTick`
  (params (DeltaSeconds :type "Float (single-precision)"))
  ;[1 1 1] Rotation
  (`SceneComponent.K2_AddWorldRotation` (`self.StaticMesh`) (`KismetMathLibrary.MakeRotator` 0.0 0.0 (`KismetMathLibrary.RandomFloatInRange` 1.0 2.0)) false false))

(event `Move To Location`
  (params (Duration :type "Float (single-precision)") (`Target Location` :type "Vector Structure"))
  ;[1 1 1] 注释
  (`KismetSystemLibrary.Delay` Duration)
  (bind _output_get (set `self.Target Location` `Target Location`))
  (bind (_direction _track_01) (`Timeline|TimeLine`)
    (:`Update`
      (`self.K2_SetActorLocation` (`KismetMathLibrary.VLerp` (`self.K2_GetActorLocation`) _output_get _track_01)))))

(event `Move to Target`
  (params (Duration :type "Float (single-precision)"))
  (bind _target (`self.Target`))
  ;[1 1 1] 注释
  (`/Engine/EditorBlueprintResources/StandardMacros.IsValid` _target
    (:`Is Valid`
      (`KismetSystemLibrary.Delay` Duration)
      (bind _output_get (set `self.Target Location` (`self.K2_GetActorLocation` _target)))
      (bind (_direction _track_01) (`Timeline|TimeLine_01`)
        (:`Update`
          (`self.K2_SetActorLocation` (`KismetMathLibrary.VLerp` (`self.K2_GetActorLocation`) _output_get _track_01)))))))

(event `self.Sphere.OnComponentBeginOverlap`
  (params (OverlappedComponent :type "PrimitiveComponent Object Reference") (OtherActor :type "Actor Object Reference") (OtherComp :type "PrimitiveComponent Object Reference") (OtherBodyIndex :type Integer) (bFromSweep :type Boolean) (SweepResult :type "HitResult Structure (by ref)"))
  ;[1 1 1] DestroyActor
  (bind _asbp_top_down_character (cast `/Game/Blueprints/Character/BP_TopDownCharacter` OtherActor))
  (`/Game/Blueprints/Character/BP_TopDownCharacter.AddXP` _asbp_top_down_character (`self.XP`))
  (`self.K2_DestroyActor`))

(fn `UserConstructionScript`)