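; BP_GenerateRewards is an actor that scatters XP pickups around its location.
; Half a second after BeginPlay, it spawns a set Number of BP_Dropped_XP actors at its position with random yaw and stores them in an array.
; It immediately sends each one via MoveToLocation to a random reachable navmesh point within Radius.
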(event `self.ReceiveBeginPlay`
  (`KismetSystemLibrary.Delay` 0.5)
  (for _ (range (`self.Number`))
    (bind _returnvalue (`|SpawnActorFromClass` "/Game/Blueprints/XP/BP_Dropped_XP.BP_Dropped_XP_C" (`KismetMathLibrary.MakeTransform` (`self.K2_GetActorLocation`) (`KismetMathLibrary.MakeRotator` 0.0 0.0 (`KismetMathLibrary.RandomFloatInRange` 0.0 360.0))) "Undefined" "MultiplyWithRoot" null null null))
    (`KismetArrayLibrary.Array_Add` (`self.Array`) _returnvalue)
    (`/Game/Blueprints/XP/BP_Dropped_XP.Move To Location` _returnvalue 0.0 (`NavigationSystemV1.K2_GetRandomReachablePointInRadius` (`self.K2_GetActorLocation`) (`self.Radius`) null null))))

(fn `UserConstructionScript`)