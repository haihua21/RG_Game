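; XP reward dropper actor that spawns a set number of dropped XP pickups and sends them to the player on pickup.
; On BeginPlay it finds the top-down character as target and scatters the pickups to random reachable nav points within a radius.
; When the character enters the trigger sphere, a delayed, re-entrant loop calls MoveToTarget on stored pickups, destroying the dropper upon hitting an invalid one.
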(event `self.ReceiveBeginPlay`
  (bind _radius (`self.Radius`))
  (bind _returnvalue (* _radius -1.0))
  ;[1 1 1] Dropped
  (bind _returnvalue_2 (`GameplayStatics.GetActorOfClass` "/Game/Blueprints/Character/BP_TopDownCharacter.BP_TopDownCharacter_C"))
  (set `self.Actor_Target` _returnvalue_2)
  (`SphereComponent.SetSphereRadius` (`self.Sphere`) (`self.CollierRadius`) true)
  (for _ (range (`self.Number`))
    (bind _returnvalue_3 (`|SpawnActorFromClass` "/Game/Blueprints/XP/Bp1_Dropped_XP.Bp1_Dropped_XP_C" (`KismetMathLibrary.MakeTransform` (`self.K2_GetActorLocation`) (`KismetMathLibrary.MakeRotator` 0.0 0.0 (`KismetMathLibrary.RandomFloatInRange` 0.0 360.0))) "Undefined" "MultiplyWithRoot" null (`self.Actor_Target`) null))
    (`KismetArrayLibrary.Array_Add` (`self.Array`) _returnvalue_3)
    (bind _output_get (set `self.XP_Actor` _returnvalue_3))
    (`/Engine/EditorBlueprintResources/StandardMacros.IsValid` _output_get
      (:`Is Valid`
        (`/Game/Blueprints/XP/Bp1_Dropped_XP.Move To Location` _output_get 0.2 (`NavigationSystemV1.K2_GetRandomReachablePointInRadius` (- (`self.K2_GetActorLocation`) (`KismetMathLibrary.MakeVector` (`KismetMathLibrary.RandomFloatInRange` _returnvalue _radius) (`KismetMathLibrary.RandomFloatInRange` _returnvalue _radius) (`KismetMathLibrary.RandomFloatInRange` -30.0 30.0))) (`self.Radius`) null null))))))

(event `self.Sphere.OnComponentBeginOverlap`
  (params (OverlappedComponent :type "PrimitiveComponent Object Reference") (OtherActor :type "Actor Object Reference") (OtherComp :type "PrimitiveComponent Object Reference") (OtherBodyIndex :type Integer) (bFromSweep :type Boolean) (SweepResult :type "HitResult Structure (by ref)"))
  ;[1 1 1] 拾取，可以外部调用
  (`/Engine/EditorBlueprintResources/StandardMacros.IsValid` (`self.XP_Actor`) :!label _label
    (:`Is Valid`
      (cast `/Game/Blueprints/Character/BP_TopDownCharacter` OtherActor)
      (`KismetSystemLibrary.Delay` 0.2)
      (for _array_element (`self.Array`)
        (`/Engine/EditorBlueprintResources/StandardMacros.IsValid` _array_element
          (:`Is Valid`
            (`/Game/Blueprints/XP/Bp1_Dropped_XP.Move to Target` _array_element 0.0)
            (goto _label))
          (:`Is Not Valid`
            (`self.K2_DestroyActor`)))))))

(fn `UserConstructionScript`)