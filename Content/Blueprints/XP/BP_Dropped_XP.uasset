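; BP_Dropped_XP is a dropped XP actor that glides to a destination after a delay.
; MoveToLocation takes a fixed point, while MovetoTarget checks that Target is valid before the delay, then samples its position once afterward.
; Each uses its own timeline to lerp from the actor's current location every update, without sweep, so the target is not tracked while moving.
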(event `Move To Location`
  (params (Duration :type "Float (single-precision)") (`Target Location` :type "Vector Structure"))
  (`KismetSystemLibrary.Delay` Duration)
  (bind _output_get (set `self.Target Location` `Target Location`))
  (bind (_direction _track_01) (`Timeline|TimeLine`)
    (:`Update`
      (`self.K2_SetActorLocation` (`KismetMathLibrary.VLerp` (`self.K2_GetActorLocation`) _output_get _track_01)))))

(event `Move to Target`
  (params (Duration :type "Float (single-precision)"))
  (bind _target (`self.Target`))
  (`/Engine/EditorBlueprintResources/StandardMacros.IsValid` _target
    (:`Is Valid`
      (`KismetSystemLibrary.Delay` Duration)
      (bind _output_get (set `self.Target Location` (`self.K2_GetActorLocation` _target)))
      (bind (_direction _track_01) (`Timeline|TimeLine_01`)
        (:`Update`
          (`self.K2_SetActorLocation` (`KismetMathLibrary.VLerp` (`self.K2_GetActorLocation`) _output_get _track_01)))))))

(fn `UserConstructionScript`)